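; BP_BaseItem is an item Blueprint that shows a dialogue widget when clicked through its MouseInteractionComponent.
; The click handler asks the UI subsystem for an existing widget of its UI type and toggles its visibility.
; If none exists, CreateUI creates a WBP_DialogueWidget and registers it with the subsystem.
; Both paths then pass the CharacterID and stored CreateWidget reference to SetDialogueTextInfo.
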(event `self.MouseInteractionComponent.OnMouseClickEvent`
  (params (Actor :type "Actor Object Reference"))
  (`/Engine/EditorBlueprintResources/StandardMacros.IsValid` (`self.GetUISubsystem`)
    (:`Is Valid`
      (bind _returnvalue (`UIManagerSubsystem.GetCheckUICreated` (`self.GetUISubsystem`) (`self.UIType`)))
      (`/Engine/EditorBlueprintResources/StandardMacros.IsValid` _returnvalue
        (:`Is Valid`
          (set `self.GainWdiget` _returnvalue)
          (bind _returnvalue_2 (`UIWidgetBase.IsUIVisible` (`self.GainWdiget`)))
          (`UIManagerSubsystem.SetShowUI` (`self.GetUISubsystem`) (`self.UIType`) (not _returnvalue_2) false)
          (`self.SetDialogueTextInfo` (`self.Character ID`) (`self.CreateWidget`)))
        (:`Is Not Valid`
          (`self.CreateUI`)
          (`self.SetDialogueTextInfo` (`self.Character ID`) (`self.CreateWidget`)))))
    (:`Is Not Valid`
      (`KismetSystemLibrary.LogString` "Subsystem Not Valid"))))

(fn `CreateUI`
  (locals (Visible :type Boolean :default true))
  (bind _returnvalue (`|CreateWidget` "/Game/Widgets/WBP_DialogueWidget.WBP_DialogueWidget_C"))
  (`/Engine/EditorBlueprintResources/StandardMacros.IsValid` _returnvalue
    (:`Is Valid`
      (set `self.CreateWidget` _returnvalue)
      (`UIManagerSubsystem.AddUIInfo` (`self.GetUISubsystem`) (`self.CreateWidget`) (`local.Visible`)))
    (:`Is Not Valid`
      (`KismetSystemLibrary.LogString` "Item::WidgetCreateFail"))))

(fn `UserConstructionScript`)